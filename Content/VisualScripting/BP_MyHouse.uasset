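; BP_MyHouse is an early, unfinished Blueprint that begins assembling a house from runtime-created components, starting with the foundation.
; BeginPlay prints a start message and adds three static mesh components, configuring only the first, with no mesh assigned and zero scale.
; The construction script is empty, and the array and map nodes are disconnected experiments that never affect the build.
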(event EventBeginPlay
  ;[1 1 1] Fondation
  (Development|PrintString "Start Construction")
  (bind _returnvalue (AddComponent|AddStaticMeshComponent false))
  (Components|StaticMesh|SetStaticMesh _returnvalue 0)
  (Transformation|SetRelativeLocation _returnvalue "0, 0, 0" false false)
  (Transformation|SetRelativeScale3D _returnvalue "0, 0, 0")
  (AddComponent|AddStaticMeshComponent false (Math|Transform|MakeTransform "0, 0, 0"))
  (AddComponent|AddStaticMeshComponent false))

(fn ConstructionScript)